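; T1_Tube_BP is a teleport tube that moves the player character to a linked destination on a key press.
; Box overlap by MyCharacter enables input and arms a teleport flag.
; Pressing C while armed sets the character's location to the TargetLocation Arrow, then disarms after a short delay.
; Ending overlap calls DisableInput and clears the flag, with debug prints reporting each state.
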(event `self.Box.OnComponentBeginOverlap`
  (params (OverlappedComponent :type "PrimitiveComponent Object Reference") (OtherActor :type "Actor Object Reference") (OtherComp :type "PrimitiveComponent Object Reference") (OtherBodyIndex :type Integer) (bFromSweep :type Boolean) (SweepResult :type "HitResult Structure (by ref)"))
  ;[1 1 1] Overlab and Enable Input
  (bind _asmy_character (cast `/Game/Blueprint/MyCharacter` OtherActor))
  (`KismetSystemLibrary.PrintString` "Teleport Enabled")
  (`self.EnableInput` (`GameplayStatics.GetPlayerController` 0))
  (set `self.EnableTeleport` true))

(event `Key|C`
  (params (Key :type "Key Structure"))
  ;[1 0.4876 0.7144] Press 'C' Check Condition Then Set New World Location
  (:`Pressed`
    (if (`self.EnableTeleport`)
      (`SceneComponent.K2_SetWorldLocation` (`Actor.RootComponent` (stale `self.Box.OnComponentBeginOverlap` _asmy_character)) (`SceneComponent.K2_GetComponentLocation` (`/Game/Blueprint/T1_Tube_BP.Arrow` (`self.TargetLocation`))) false false)
      (`KismetSystemLibrary.Delay` 1.0)
      (set `self.EnableTeleport` false)
      (`KismetSystemLibrary.PrintString` "Teleport End"))))

(event `self.Box.OnComponentEndOverlap`
  (params (OverlappedComponent :type "PrimitiveComponent Object Reference") (OtherActor :type "Actor Object Reference") (OtherComp :type "PrimitiveComponent Object Reference") (OtherBodyIndex :type Integer))
  ;[0.5796 1 0.6636] End Overlap Then Disable Input
  (`self.DisableInput` (`GameplayStatics.GetPlayerController` 0) null)
  (set `self.EnableTeleport` false)
  (`KismetSystemLibrary.PrintString` "TeleportDisabled"))

(fn `UserConstructionScript`)