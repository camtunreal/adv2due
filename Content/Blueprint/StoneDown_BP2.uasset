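; A falling stone hazard Blueprint, using Super Mario Bros. 3 object sprites, that repeatedly runs a drop animation.
; After a short delay on BeginPlay, a timeline lerps the sprite's relative location between points A and B, then restarts itself after a pause.
; The same timeline value swaps the sprite's face once it passes a threshold near the end of the lerp.
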(event `self.ReceiveBeginPlay`
  ;[1 1 1] Start
  (`KismetSystemLibrary.Delay` 1.0)
  ;;[0.2652 0.7201 1] Call DropStone Event
  (`self.DropStone`))

(event `DropStone`
  ;[0.5696 1 0.5388] DropStone Script
  ;;[0.2824 0.8706 0.9216] DropStone Event
  (bind (_direction _speed) (`Timeline|Timeline_Animation` :`NewTime` 0.0 :!via `PlayFromStart`)
    (:`Update`
      (`|ExecutionSequence`
        (:`then_0`
          (`SceneComponent.K2_SetRelativeLocation` (`self.PaperSprite`) (`KismetMathLibrary.VLerp` (`self.A`) (`self.B`) _speed) false false))
        (:`then_1`
          (`self.Changing Faces`))))
    (:`Finished`
      (`KismetSystemLibrary.Delay` 1.0)
      ;;[0.2824 0.8706 0.9216] Call DropStone again
      (`self.DropStone`))))

(event `Changing Faces`
  (bind _papersprite (`self.PaperSprite`))
  ;[0.4471 0.2854 1] Changing Faces
  (if (>= (stale `DropStone` _speed) 0.8)
    (`PaperSpriteComponent.SetSprite` _papersprite "/Game/Asset2_Mario/SMB3_Objects_Sprite_388.SMB3_Objects_Sprite_388")
    (else
      (`PaperSpriteComponent.SetSprite` _papersprite "/Game/Asset2_Mario/SMB3_Objects_Sprite_371.SMB3_Objects_Sprite_371"))))

(fn `UserConstructionScript`)