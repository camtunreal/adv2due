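; Warp pipe actor that teleports the player character to a linked target location when C is pressed inside its trigger box.
; Box overlap with MyCharacter enables input and arms the warp; leaving disables both.
; Warping moves the character's root component to the target's Arrow position without sweep, starts a one-second camera fade from full opacity, and clears the warp flag after a delay.
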(event `self.Box.OnComponentBeginOverlap`
  (params (OverlappedComponent :type "PrimitiveComponent Object Reference") (OtherActor :type "Actor Object Reference") (OtherComp :type "PrimitiveComponent Object Reference") (OtherBodyIndex :type Integer) (bFromSweep :type Boolean) (SweepResult :type "HitResult Structure (by ref)"))
  ;[1 1 1] Enable Input
  (bind _asmy_character (cast `/Game/Blueprint/MyCharacter` OtherActor))
  (`KismetSystemLibrary.PrintString` "Enable Input")
  (`self.EnableInput` (`GameplayStatics.GetPlayerController` 0))
  (set `self.EnableWarp` true))

(event `Key|C`
  (params (Key :type "Key Structure"))
  ;[1 1 1] Warp
  (:`Pressed`
    (if (`self.EnableWarp`)
      (`SceneComponent.K2_SetWorldLocation` (`Actor.RootComponent` (stale `self.Box.OnComponentBeginOverlap` _asmy_character)) (`SceneComponent.K2_GetComponentLocation` (`/Game/Blueprint/WarpPipe_BP.Arrow` (`self.TargetLocation`))) false false)
      (`|ExecutionSequence`
        (:`then_0`
          (`KismetSystemLibrary.Delay` 1.0)
          (set `self.EnableWarp` false)
          (`KismetSystemLibrary.PrintString` "Teleport Finish"))
        (:`then_1`
          (`PlayerCameraManager.StartCameraFade` :`self` (`GameplayStatics.GetPlayerCameraManager` 0) :`FromAlpha` 1.0 :`Duration` 1.0))))))

(event `self.Box.OnComponentEndOverlap`
  (params (OverlappedComponent :type "PrimitiveComponent Object Reference") (OtherActor :type "Actor Object Reference") (OtherComp :type "PrimitiveComponent Object Reference") (OtherBodyIndex :type Integer))
  (cast `/Game/Blueprint/MyCharacter` OtherActor)
  (`self.DisableInput` (`GameplayStatics.GetPlayerController` 0))
  (set `self.EnableWarp` false)
  (`KismetSystemLibrary.PrintString` "Disable Warp"))

(fn `UserConstructionScript`)